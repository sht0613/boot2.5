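; BP_Weapon is a weapon actor that attaches to a character and damages actors it overlaps.
; B_AttachToCharacter stores the owning character and attaches the weapon to the "shield" socket on that character's mesh.
; B_DoDamage checks the Weapon component's overlaps when called and applies fixed damage to the first actor other than the owner, crediting the owner's controller as instigator.
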(fn `B_AttachToCharacter`
  (params (character :type "Character Object Reference"))
  (returns (bResult :type Boolean))
  (bind _output_get (set `self.Character` character))
  (`self.K2_AttachToComponent` (`Character.Mesh` _output_get) "shield" "KeepRelative" "KeepRelative" "KeepRelative")
  (return true))

(fn `B_DoDamage`
  (returns (Result :type Boolean))
  (bind _character (`self.Character`))
  (for _array_element (`PrimitiveComponent.GetOverlappingActors` (`self.Weapon`) "/Script/Engine.Actor")
    (if (!= _array_element _character)
      (`GameplayStatics.ApplyDamage` _array_element 25.0 (`Pawn.GetController` _character) self)
      (return true))))

(fn `UserConstructionScript`)