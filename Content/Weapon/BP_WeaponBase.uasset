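; Base weapon Blueprint that a character can hold, drop and attack with.
; Attaching stores the Character, disables physics on the Weapon component and snaps to a socket on the character mesh; detaching reverses this.
; Attacking plays an attack montage on the holder.
; A separate damage function checks actors overlapping the Weapon and applies fixed damage to the first one other than the holder, crediting its controller.
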(fn `B_AttachToCharacter`
  (params (character :type "Character Object Reference"))
  (returns (bResult :type Boolean))
  (bind _output_get (set `self.Character` character))
  (`PrimitiveComponent.SetSimulatePhysics` (`self.Weapon`) false)
  (`self.K2_AttachToComponent` (`Character.Mesh` _output_get) (`self.Socket Name`) "SnapToTarget" "SnapToTarget" "SnapToTarget")
  (return true))

(fn `B_DetachToCharacter`
  (params (Character :type "Character Object Reference"))
  (returns (BResult :type Boolean))
  (`self.K2_DetachFromActor` "KeepWorld" "KeepWorld" "KeepWorld")
  ; 기능: Target컴포넌트에 적용할 물리 시뮬레이션을 끄고,켜기 위해
  ; ex)무기를 잡을때는 oFF/ 무기를 놓을 때는 ON할때 많으니까 쉽게 조절할려고
  (`PrimitiveComponent.SetSimulatePhysics` (`self.Weapon`) true)
  (set `self.Character` null)
  (return false))

(fn `B_DoAttack`
  (returns (BResult :type Boolean))
  (`Character.PlayAnimMontage` (`self.Character`) "/Game/Characters/Mannequins/Animations/Attack/AM_WeaponAttack.AM_WeaponAttack" 1.0 "None")
  (return false))

(fn `B_DoDamage`
  (returns (Result :type Boolean))
  (bind _character (`self.Character`))
  (for _array_element (`PrimitiveComponent.GetOverlappingActors` (`self.Weapon`) "/Script/Engine.Actor")
    (if (!= _array_element _character)
      (`GameplayStatics.ApplyDamage` _array_element 25.0 (`Pawn.GetController` _character) self)
      (return true))))

(fn `UserConstructionScript`)