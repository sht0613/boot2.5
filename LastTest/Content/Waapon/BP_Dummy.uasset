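; BP_Dummy is a damageable dummy actor with monster stats and a name tag that shatters when its HP runs out.
; On BeginPlay it copies its DT_Monster row into MonState and creates a viewport widget showing name and HP.
; AnyDamage lowers HP and refreshes the tag.
; Death crumbles the Geometry Collection with a radial impulse, removes the tag and destroys the actor after a timed delay.
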(event `self.ReceiveBeginPlay`
  (`|ExecutionSequence`
    (:`then_0`
      (bind _returnvalue (`|GetDataTableRow` "/Game/Waapon/DT_Monster.DT_Monster" (`self.Row Name`))
        (:`then`
          (setmembers `/Game/Waapon/ST_CurMonState` :`StructRef` (`self.MonState`) :`State` _returnvalue :`CurHP` (`.MaxHP_6_2A65D0D64190FCACDCE273B88A8D92D8` (break `/Game/Waapon/ST_Monstate` _returnvalue))))))
    (:`then_1`
      (`self.CreateNameTag`))))

(event `self.ReceiveAnyDamage`
  (params (Damage :type "Float (single-precision)") (DamageType :type "DamageType Object Reference") (InstigatedBy :type "Controller Object Reference") (DamageCauser :type "Actor Object Reference"))
  (bind _isjustdeath (`self.addDamage` Damage))
  (if _isjustdeath
    (`self.Do_Death`)))

(fn `addDamage`
  (params (Damage :type "Float (double-precision)"))
  (returns (IsJustDeath :type Boolean))
  (bind (_monstate_state _monstate_curhp) (break `/Game/Waapon/ST_CurMonState` (`self.MonState`)))
  (if (`self.isDeath`)
    (return false)
    (else
      (setmembers `/Game/Waapon/ST_CurMonState` :`StructRef` (`self.MonState`) :`CurHP` (- _monstate_curhp Damage))
      (`self.UpdateHP`)
      (return (`self.isDeath`)))))

(fn `CreateNameTag`
  (bind _returnvalue (`|CreateWidget` "/Game/Waapon/NameTagWidget.NameTagWidget_C" null self))
  (bind _output_get (set `self.NameTag` _returnvalue))
  (`UserWidget.AddToViewport` _output_get 0)
  (`self.UpdateName`)
  (`self.UpdateHP`))

(fn `Do_Death`
  (bind _geometrycollection (`self.GeometryCollection`))
  (`GeometryCollectionComponent.CrumbleActiveClusters` _geometrycollection)
  (`PrimitiveComponent.AddRadialImpulse` _geometrycollection (+ (`SceneComponent.K2_GetComponentLocation` _geometrycollection) (0.0 0.0 30.0)) 15.0 10000.0 "RIF_Constant" false)
  (`Widget.RemoveFromParent` (`self.NameTag`))
  (`KismetSystemLibrary.K2_SetTimer` null "Do_Destroy" 5.0))

(fn `Do_Destroy`
  (`self.K2_DestroyActor`))

(fn `isDeath`
  (returns (isDeath :type Boolean))
  (bind (_monstate_state _monstate_curhp) (break `/Game/Waapon/ST_CurMonState` (`self.MonState`)))
  (return (<= _monstate_curhp 0.0)))

(fn `NameTag_HP`
  (returns (CurHP :type "Float (double-precision)") (MaxHP :type "Float (double-precision)"))
  (bind _monstate (`self.MonState`))
  (return (`.CurHP_4_C45B545A456CB7796AF032915F30124D` (break `/Game/Waapon/ST_CurMonState` _monstate)) (`.MaxHP_6_2A65D0D64190FCACDCE273B88A8D92D8` (break `/Game/Waapon/ST_Monstate` (break `/Game/Waapon/ST_CurMonState` _monstate)))))

(fn `NameTag_Location`
  (returns (WorldLoc :type "Vector Structure"))
  (return (`SceneComponent.K2_GetComponentLocation` (`self.NameTagLoc`))))

(fn `NameTag_Name`
  (returns (Name :type String))
  (return (break `/Game/Waapon/ST_Monstate` (break `/Game/Waapon/ST_CurMonState` (`self.MonState`)))))

(fn `UpdateHP`
  (bind _monstate (`self.MonState`))
  (bind _nametag (`self.NameTag`)
    (:`then`
      (`/Game/Waapon/NameTagWidget.SetNameTagHP` _nametag (`.CurHP_4_C45B545A456CB7796AF032915F30124D` (break `/Game/Waapon/ST_CurMonState` _monstate)) (`.MaxHP_6_2A65D0D64190FCACDCE273B88A8D92D8` (break `/Game/Waapon/ST_Monstate` (break `/Game/Waapon/ST_CurMonState` _monstate)))))
    (:`else`)))

(fn `UpdateName`
  (`/Game/Waapon/NameTagWidget.SetNameTagName` (`self.NameTag`) (break `/Game/Waapon/ST_Monstate` (break `/Game/Waapon/ST_CurMonState` (`self.MonState`)))))

(fn `UserConstructionScript`)