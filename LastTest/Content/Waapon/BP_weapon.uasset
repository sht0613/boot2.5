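; BP_weapon is a melee weapon actor that a character can carry, swing and drop.
; Attach stores the character, disables physics and snaps the weapon to a mesh socket, while detach releases it, restores physics and clears the reference.
; Attack plays a montage on the stored character.
; A separate damage function applies fixed damage to the first actor overlapping the weapon other than its holder, with the holder's controller as instigator.
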(fn `B_AttachToCharacter`
  (params (Character :type "Character Object Reference"))
  (returns (Result :type Boolean))
  (bind _output_get (set `self.Character` Character))
  (`PrimitiveComponent.SetSimulatePhysics` (`self.Weapon`) false)
  (`self.K2_AttachToComponent` (`Character.Mesh` _output_get) (`self.Socket Name`) "SnapToTarget" "SnapToTarget" "SnapToTarget")
  (return true))

(fn `B_DettachToCharacter`
  (params (Character :type "Character Object Reference"))
  (returns (BResult :type Boolean))
  (`self.K2_DetachFromActor` "KeepWorld" "KeepWorld" "KeepWorld")
  (`PrimitiveComponent.SetSimulatePhysics` (`self.Weapon`) true)
  (set `self.Character` null)
  (return false))

(fn `B_DoAttack`
  (returns (BResult :type Boolean))
  (`Character.PlayAnimMontage` (`self.Character`) "/Game/Characters/Mannequins/Animations/attack/AM_Anim_Attack.AM_Anim_Attack" 1.0 "None")
  (return false))

(fn `Do_Damage`
  (returns (Result :type Boolean))
  (bind _character (`self.Character`))
  (for _array_element (`PrimitiveComponent.GetOverlappingActors` (`self.Weapon`) "/Script/Engine.Actor")
    (if (!= _array_element _character)
      (`GameplayStatics.ApplyDamage` _array_element 30.0 (`Pawn.GetController` _character) self)
      (return true))))

(fn `UserConstructionScript`)